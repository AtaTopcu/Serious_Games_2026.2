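; BP_Dog is an interactable dog actor that the player picks up.
; It is always interactable, reports a fixed interaction type, and shows or hides its widget as a prompt.
; Interacting sets HasDog on the player and destroys the actor.
; The start and stop thrash annihilation functions are stubs that return false.
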(fn ConstructionScript)

(fn CanInterract
  (return true))

(fn GetInterractionType
  (return "NewEnumerator0"))

(fn HideInterract
  (Development|SetHiddeninGame (Variables|Default|GetWidget) true false)
  (return true))

(fn Interract
  (params (Player :type BP%20First%20Person%20Character%20Object%20Reference))
  (Variables|/Game/Blueprints/FirstPersonBP/BP_FirstPersonCharacter.BP_FirstPersonCharacter_C|SetHasDog Player true)
  (Actor|DestroyActor)
  (return true))

(fn ShowInterract
  (Development|SetHiddeninGame (Variables|Default|GetWidget) false false)
  (return true))

(fn StartThrashAnnilation
  (return false))

(fn StopThrashAnnilation
  (return false))