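; BP_ThrashAnnihilator is an interactable trash disposal prop that animates a mesh open and shut as its interaction prompt appears and disappears.
; ShowInterract reveals the Widget and calls Open; HideInterract hides it and calls Close.
; Open and Close play and reverse a Timeline, with the pitch update on StaticMesh1 wired only from Open.
; Interract and the start/stop annihilation functions are stubs returning false.
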(event Custom|Close
  (bind _newtrack_0 (Timeline|Timeline Reverse)
    (:Update
      (Transformation|SetRelativeRotation (Variables|Default|GetStaticMesh1) (Math|Rotator|MakeRotator 0.0 _newtrack_0 0.0) false false))))

(event Custom|Open
  (bind _newtrack_0 (Timeline|Timeline Play)
    (:Update
      (Transformation|SetRelativeRotation (Variables|Default|GetStaticMesh1) (Math|Rotator|MakeRotator 0.0 _newtrack_0 0.0) false false))))

(fn ConstructionScript)

(fn CanInterract
  (return true))

(fn GetInterractionType
  (return "NewEnumerator2"))

(fn HideInterract
  (Development|SetHiddeninGame (Variables|Default|GetWidget) true false)
  (CallFunction|Close)
  (return true))

(fn Interract
  (params (Player :type BP%20First%20Person%20Character%20Object%20Reference))
  (return false))

(fn ShowInterract
  (Development|SetHiddeninGame (Variables|Default|GetWidget) false false)
  (CallFunction|Open)
  (return false))

(fn StartThrashAnnilation
  (return false))

(fn StopThrashAnnilation
  (return false))