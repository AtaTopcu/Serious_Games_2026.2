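; Interactable trash pickup that gives the interacting actor a random crafting-style material: silver, plastic or circuit, in a random small quantity.
; The construction script picks the sphere component's mesh and material from TrashType, which has no effect on the item granted.
; Interact rolls the item and passes it to the caller's BPInventoryComponent, destroying the trash a tick later if the transfer succeeds.
; Its own inventory component initializes as non-player without a widget.
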(event EventBeginPlay
  (Default|EventInitilize (Variables|Default|GetBP_Inventory_Component) false false))

(event EventInteract
  (params (Calling_Actor :type BP%20First%20Person%20Character%20Object%20Reference))
  (bind _transaction_successful1 (Default|ItemTransferFunction (Variables|/Game/Blueprints/FirstPersonBP/BP_FirstPersonCharacter.BP_FirstPersonCharacter_C|GetBP_Inventory_Component Calling_Actor) (Utilities|Struct|MakeST_Item_Base (Utilities|Select :Index (Math|Random|RandomIntegerinRange 0 2) :Option%200 "silver" :Option%201 "plastic" :Option%202 "circuit") (Math|Random|RandomIntegerinRange 1 8))))
  (if _transaction_successful1
    (Utilities|FlowControl|DelayUntilNextTick)
    (Actor|DestroyActor)))

(fn ConstructionScript
  (bind _sphere (Variables|Default|GetSphere))
  (bind _trash_type (Variables|Default|GetTrash_Type))
  (Components|StaticMesh|SetStaticMesh _sphere (Utilities|Select :Index _trash_type :Option%200 "/Game/assets/broken_can.broken_can" :Option%201 "/Game/assets/Chips.Chips" :Option%202 "/Game/assets/DrinkCup.DrinkCup" :Option%203 "/Game/assets/Object_8_001.Object_8_001" :Option%204 "/Game/assets/PlasticBottle.PlasticBottle" :Option%205 "/Game/assets/trash.trash"))
  (Rendering|Material|SetMaterial _sphere 0 (Utilities|Select :Index _trash_type :Option%200 "/Game/materials/M_Can_Broken.M_Can_Broken" :Option%201 "/Game/materials/M_Cips.M_Cips" :Option%202 "/Game/materials/M_Cup.M_Cup" :Option%203 "/Game/materials/M_Can.M_Can" :Option%204 "/Game/materials/M_Plastic_Bottle.M_Plastic_Bottle" :Option%205 "/Game/materials/M_Trash.M_Trash")))