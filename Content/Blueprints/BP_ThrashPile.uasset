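; Interactable trash pile in big (dog) or small (cat) variants, broken up by the matching animal when the player has it.
; Construction sets scale, material and animal mesh from Big, and the prompt widget shows the required animal.
; Interacting reveals the animal and a timeline moves it into the pile, then DestoryPile destroys the actor.
; Big piles scatter new piles, small ones DT_Thrash items, via line traces between random navmesh points.
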(event Custom|SpawnAnimal
  (Variables|Default|SetLocation (.location (Variables|Default|GetCatOrDog)))
  (Development|SetHiddeninGame (Variables|Default|GetSkeletalMesh) false false)
  (bind _newtrack_0 (Timeline|Timeline PlayFromStart)
    (:Update
      (Transformation|SetRelativeLocation (Variables|Default|GetSkeletalMesh) (Math|Vector|Lerp(Vector) (Variables|Default|GetLocation) (Variables|/Script/Engine.SceneComponent|GetRelativeLocation (Variables|Default|GetStaticMesh)) _newtrack_0) false false))
    (:Finished
      (CallFunction|DestoryPile))))

(event EventBeginPlay
  (Appearance|SetBrushfromTexture (Variables|/Game/Blueprints/Inventory_System/Widgets/WBP_InterractionWidget1.WBP_InterractionWidget1_C|GetImage_0 (.AsWBP%20Interraction%20Widget%201 (Utilities|Casting|CastToWBP_InterractionWidget1 (UserInterface|GetWidget (Variables|Default|GetWidget))))) (select (Variables|Default|GetBig) "/Game/assets/UI/Dog.Dog" "/Game/assets/UI/Cat.Cat") false))

(fn ConstructionScript
  (bind _staticmesh (Variables|Default|GetStaticMesh))
  (Transformation|SetWorldScale3D _staticmesh (select (Variables|Default|GetBig) "1.200000,1.200000,1.200000" "0.800000,0.800000,0.800000"))
  (Rendering|Material|SetMaterial _staticmesh 0 (select (Variables|Default|GetBig) "/Game/materials/M_Trash2.M_Trash2" "/Game/materials/M_Trash.M_Trash"))
  (Transformation|SetRelativeTransform (Variables|Default|GetSkeletalMesh) (Variables|Default|GetCatOrDog) false false)
  (Components|SkeletalMesh|SetSkeletalMeshAsset (Variables|Default|GetSkeletalMesh) (select (Variables|Default|GetBig) "/Game/assets/DAWG.DAWG" "/Game/assets/CAWD.CAWD")))

(fn DestoryPile
  (bind _returnvalue (Transformation|GetActorLocation))
  (bind _player (Variables|Default|GetPlayer))
  (bind _randomlocation (AI|Navigation|GetRandomReachablePointinRadius _returnvalue 6e+02 0 0))
  (for _index (range 0 (select (Variables|Default|GetBig) 5 10))
    (bind _outhit (Collision|LineTraceByChannel _randomlocation (- _randomlocation "0.000000,0.000000,100.000000") "TraceTypeQuery1" false 0 "None"))
    (bind _outrownames (DataTable|GetDataTableRowNames "/Game/Blueprints/DT_Thrash.DT_Thrash"))
    (bind _returnvalue_2 (Utilities|GetDataTableRow "/Game/Blueprints/DT_Thrash.DT_Thrash" (.OutItem (Utilities|Array|Random _outrownames)))
      (:then
        (if (Variables|Default|GetBig)
          (Game|SpawnActorfromClass "BP_ThrashPile_C" (Math|Transform|MakeTransform (.Location (Collision|BreakHitResult _outhit)) "0, 0, 0" "1.000000,1.000000,1.000000") "Undefined" "MultiplyWithRoot" 0 0)
          (else
            (Game|SpawnActorfromClass "/Game/Blueprints/BP_Thrash.BP_Thrash_C" (Math|Transform|MakeTransform (.Location (Collision|BreakHitResult _outhit)) "0, 0, 0" "1.000000,1.000000,1.000000") "Undefined" "MultiplyWithRoot" 0 _returnvalue_2 0))))))
  (if (Variables|Default|GetBig)
    (Variables|/Game/Blueprints/FirstPersonBP/BP_FirstPersonCharacter.BP_FirstPersonCharacter_C|SetHasDog _player true)
    (else
      (Variables|/Game/Blueprints/FirstPersonBP/BP_FirstPersonCharacter.BP_FirstPersonCharacter_C|SetHasCat _player true)))
  (Actor|DestroyActor))

(fn CanInterract
  (return true))

(fn GetInterractionType
  (return "NewEnumerator0"))

(fn HideInterract
  (Rendering|SetVisibility (Variables|Default|GetWidget) false false)
  (return false))

(fn Interract
  (params (Player :type BP%20First%20Person%20Character%20Object%20Reference))
  (bind _output_get (Variables|Default|SetPlayer Player))
  (if (select (Variables|Default|GetBig) (Variables|/Game/Blueprints/FirstPersonBP/BP_FirstPersonCharacter.BP_FirstPersonCharacter_C|GetHasDog _output_get) (Variables|/Game/Blueprints/FirstPersonBP/BP_FirstPersonCharacter.BP_FirstPersonCharacter_C|GetHasCat _output_get))
    (if (Variables|Default|GetBig)
      (Variables|/Game/Blueprints/FirstPersonBP/BP_FirstPersonCharacter.BP_FirstPersonCharacter_C|SetHasDog (Variables|Default|GetPlayer) true)
      (else
        (Variables|/Game/Blueprints/FirstPersonBP/BP_FirstPersonCharacter.BP_FirstPersonCharacter_C|SetHasCat (Variables|Default|GetPlayer) true)))
    (Utilities|FlowControl|DoOnce false
      (:Completed
        (CallFunction|SpawnAnimal)
        (Rendering|SetVisibility (Variables|Default|GetWidget) false false)
        (return true)))))

(fn ShowInterract
  (Rendering|SetVisibility (Variables|Default|GetWidget) true false)
  (return false))

(fn StartThrashAnnilation
  (return false))

(fn StopThrashAnnilation
  (return false))