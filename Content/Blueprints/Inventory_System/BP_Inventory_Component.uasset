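; Inventory component that holds item stacks by ID and quantity, capped by total item count and slot count.
; ItemTransferFunction sums held quantities, then merges an incoming item into a matching stack or adds a new slot, returning success.
; Transfers over the item cap always fail, as the computed partial amount is never positive.
; Initialization stores player and widget flags; the widget refresh event is an empty stub.
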(event Custom|Event_Initilize
  (params (IsPlayer? :type Boolean) (Needs_Widget? :type Boolean))
  ;[0.1604 1 0 0.5] INITILIZE
  (Variables|Default|SetIsPlayer IsPlayer?)
  (bind _output_get (Variables|Default|SetHas_Widget Needs_Widget?))
  (if _output_get
    _))

(event Custom|Update_Inventory
  ;[0.15 0.15 0.15 0.5] Update Widget inventory
)

(fn ItemTransferFunction
  (params (Item :type ST%20Item%20Base%20Structure))
  (bind _inventory (Variables|Default|GetInventory))
  (LocalVariables|SetIncoming_Item Item)
  ;[0.15 0.15 0.15 0.5] Comment
  (for _array_element (Variables|Default|GetInventory)
    (LocalVariables|SetTotal_item_count (+ (.Quantity (Utilities|Struct|BreakST_Item_Base _array_element)) (LocalVariables|GetTotal_item_count))))
  (if (>= (- (Variables|Default|GetMax_Items) (+ (LocalVariables|GetTotal_item_count) (.Quantity (Utilities|Struct|BreakST_Item_Base (LocalVariables|GetIncoming_Item))))) 0)
    (LocalVariables|SetTaken_Item_Q (.Quantity (Utilities|Struct|BreakST_Item_Base (LocalVariables|GetIncoming_Item))))
    (else
      (bind _output_get (LocalVariables|SetTaken_Item_Q (- (Variables|Default|GetMax_Items) (+ (LocalVariables|GetTotal_item_count) (.Quantity (Utilities|Struct|BreakST_Item_Base (LocalVariables|GetIncoming_Item)))))))
      (if (<= _output_get 0)
        (return false)
        (else
          _))))
  ;[0.15 0.15 0.15 0.5] step 1
  (bind (_array_element_2 _array_index) (Utilities|Array|ForEachLoopwithBreak (Variables|Default|GetInventory) :!label _label)
    (:LoopBody
      (if (== (.ID (Utilities|Struct|BreakST_Item_Base _array_element_2)) (.ID (Utilities|Struct|BreakST_Item_Base (LocalVariables|GetIncoming_Item))))
        (LocalVariables|SetItem_Found true)
        (LocalVariables|SetFound_Index _array_index)
        (goto _label Break)))
    (:Completed
      (if (LocalVariables|GetItem_Found)
        ;[0.15 0.15 0.15 0.5] Comment
        (Utilities|Array|SetArrayElem _inventory (LocalVariables|GetFound_Index) (Utilities|Struct|MakeST_Item_Base (.ID (Utilities|Struct|BreakST_Item_Base (Utilities|Array|Get(acopy) _inventory (LocalVariables|GetFound_Index)))) (+ (.Quantity (Utilities|Struct|BreakST_Item_Base (Utilities|Array|Get(acopy) _inventory (LocalVariables|GetFound_Index)))) (LocalVariables|GetTaken_Item_Q))))
        (LocalVariables|SetTransaction_Successful true)
        (elif (< (Utilities|Array|Length (Variables|Default|GetInventory)) (Variables|Default|GetMax_Slots))
          (Utilities|Array|AddUnique (Variables|Default|GetInventory) (Utilities|Struct|MakeST_Item_Base (.ID (Utilities|Struct|BreakST_Item_Base (LocalVariables|GetIncoming_Item))) (LocalVariables|GetTaken_Item_Q)))
          (LocalVariables|SetTransaction_Successful true)
          (else
            (LocalVariables|SetTransaction_Successful false))))
      (CallFunction|UpdateInventory)
      (return (LocalVariables|GetTransaction_Successful)))))