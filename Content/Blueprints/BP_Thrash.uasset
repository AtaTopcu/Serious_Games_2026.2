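; BP_Thrash is an interactable trash pickup that a player can collect.
; Its construction script sets the cube component's mesh from the STThrash data.
; Interacting passes that data to the player's CollectThrash and destroys the actor only if collection succeeds, while show and hide calls toggle the widget.
; It always allows interaction, and its start and stop annihilation functions just return false.
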(fn ConstructionScript
  (Components|StaticMesh|SetStaticMesh (Variables|Default|GetCube) (Utilities|Struct|BreakST_Thrash (Variables|Default|GetST_Thrash))))

(fn CanInterract
  (return true))

(fn GetInterractionType
  (return "NewEnumerator0"))

(fn HideInterract
  (Development|SetHiddeninGame (Variables|Default|GetWidget) true false)
  (return true))

(fn Interract
  (params (Player :type BP%20First%20Person%20Character%20Object%20Reference))
  (bind _returnvalue (Default|CollectThrash Player (Variables|Default|GetST_Thrash)))
  (if _returnvalue
    (Actor|DestroyActor)
    (return true)
    (else
      (return false))))

(fn ShowInterract
  (Development|SetHiddeninGame (Variables|Default|GetWidget) false false)
  (return true))

(fn StartThrashAnnilation
  (return false))

(fn StopThrashAnnilation
  (return false))